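; Tank Blueprint that handles player camera look controls for the tank.
; Horizontal axis input yaws the LeftRightCamera component, while vertical axis input pitches the SpringArm, splitting the two rotations across separate components.
; Both rotations are local and scale by world delta time and a SensitivityRate variable for frame-rate independent movement.
; BeginPlay, overlap, Tick and the construction script do nothing.
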(event EventBeginPlay)

(event Collision|EventActorBeginOverlap
  (params (OtherActor :type Actor%20Object%20Reference)))

(event EventTick
  (params (DeltaSeconds :type Float%20%28single-precision%29)))

(event Input|AxisEvents|InputAxisLeftRightCameraMovement
  (params (AxisValue :type Float%20%28single-precision%29))
  (Transformation|AddLocalRotation (Variables|Default|GetLeft%20Right%20Camera) (Math|Rotator|MakeRotator 0.0 0.0 (* AxisValue (Utilities|Time|GetWorldDeltaSeconds) (Variables|Default|GetSensitivity%20Rate))) false false))

(event Input|AxisEvents|InputAxisUpDownCameraMovement
  (params (AxisValue :type Float%20%28single-precision%29))
  (Transformation|AddLocalRotation (Variables|Default|GetSpringArm) (Math|Rotator|MakeRotator 0.0 (* AxisValue (Utilities|Time|GetWorldDeltaSeconds) (Variables|Default|GetSensitivity%20Rate)) 0.0) false false))

(fn ConstructionScript)